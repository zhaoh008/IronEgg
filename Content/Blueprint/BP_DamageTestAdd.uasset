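; BP_DamageTestAdd is a test volume that periodically applies the GE_DamegesAdd Gameplay Effect to characters inside its Box.
; BeginPlay starts a looping one-second timer, apparently driving the jiance detection event.
; That event polls overlapping BP_Charactor actors and, where an Ability System Component is valid, has it apply the effect spec to itself, so each character is its own effect source.
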(event `self.ReceiveBeginPlay`
  (`KismetSystemLibrary.K2_SetTimerDelegate` (`|CreateDelegate` :!event `jiance`) 1.0 true))

(event `jiance`
  (for _array_element (`PrimitiveComponent.GetOverlappingActors` (`self.Box`) "/Game/Blueprint/BP_Charactor.BP_Charactor_C")
    (bind _asbp_charactor (cast `/Game/Blueprint/BP_Charactor` _array_element))
    (bind _returnvalue (`SCharacter.GetSAbilitySystemComponent` _asbp_charactor))
    (`/Engine/EditorBlueprintResources/StandardMacros.IsValid` _returnvalue
      (:`Is Valid`
        (`AbilitySystemComponent.BP_ApplyGameplayEffectSpecToSelf` _returnvalue (`AbilitySystemComponent.MakeOutgoingSpec` _returnvalue "/Game/Blueprint/GE/GE_DamegesAdd.GE_DamegesAdd_C" 0.0 (`AbilitySystemComponent.MakeEffectContext` _returnvalue)))))))

(fn `UserConstructionScript`)