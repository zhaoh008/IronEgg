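; Character Blueprint that connects the Gameplay Ability System to an overhead-style WBP_Health widget showing health, mana and stamina.
; Server possession applies the InitGE startup effects to the ability system component, then initializes the bars.
; BeginPlay and the client PlayerState callback also initialize them, and an async attribute listener keeps them updated.
; A helper fetches the component from SPlayerState; the ability-granting event exists but its call is unwired.
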(event `授予所有技能`
  (bind _returnvalue (`self.GetSAbilitySystemComponent`))
  (`/Engine/EditorBlueprintResources/StandardMacros.IsValid` _returnvalue
    (:`Is Valid`
      (for _array_element (`self.Abilities`)
        (`AbilitySystemComponent.K2_GiveAbility` _returnvalue _array_element 0 -1)))))

(event `初始化技能效果`
  (bind _returnvalue (`self.GetSAbilitySystemComponent`))
  (`/Engine/EditorBlueprintResources/StandardMacros.IsValid` _returnvalue
    (:`Is Valid`
      (for _array_element (`self.InitGE`)
        (`AbilitySystemComponent.BP_ApplyGameplayEffectSpecToSelf` _returnvalue (`AbilitySystemComponent.MakeOutgoingSpec` _returnvalue _array_element 0.0 (`AbilitySystemComponent.MakeEffectContext` _returnvalue)))))))

(event `self.ReceiveBeginPlay`
  (bind _returnvalue (`self.GetSAbilitySystemComponent`))
  (bind (_bfound _returnvalue_2) (`AbilitySystemComponent.GetGameplayAttributeValue` _returnvalue (struct :`AttributeName` "Stamina" :`Attribute` "/Script/IronEgg.SAttributeSet:Stamina" :`AttributeOwner` "/Script/CoreUObject.Class'\"/Script/IronEgg.SAttributeSet\"'")))
  (bind (_bfound_2 _returnvalue_3) (`AbilitySystemComponent.GetGameplayAttributeValue` _returnvalue (struct :`AttributeName` "MaxMana" :`Attribute` "/Script/IronEgg.SAttributeSet:MaxMana" :`AttributeOwner` "/Script/CoreUObject.Class'\"/Script/IronEgg.SAttributeSet\"'")))
  (bind (_bfound_3 _returnvalue_4) (`AbilitySystemComponent.GetGameplayAttributeValue` _returnvalue (struct :`AttributeName` "MaxHealth" :`Attribute` "/Script/IronEgg.SAttributeSet:MaxHealth" :`AttributeOwner` "/Script/CoreUObject.Class'\"/Script/IronEgg.SAttributeSet\"'")))
  (bind (_bfound_4 _returnvalue_5) (`AbilitySystemComponent.GetGameplayAttributeValue` _returnvalue (struct :`AttributeName` "Health" :`Attribute` "/Script/IronEgg.SAttributeSet:Health" :`AttributeOwner` "/Script/CoreUObject.Class'\"/Script/IronEgg.SAttributeSet\"'")))
  (bind (_bfound_5 _returnvalue_6) (`AbilitySystemComponent.GetGameplayAttributeValue` _returnvalue (struct :`AttributeName` "Mana" :`Attribute` "/Script/IronEgg.SAttributeSet:Mana" :`AttributeOwner` "/Script/CoreUObject.Class'\"/Script/IronEgg.SAttributeSet\"'")))
  (bind (_bfound_6 _returnvalue_7) (`AbilitySystemComponent.GetGameplayAttributeValue` _returnvalue (struct :`AttributeName` "MaxStamina" :`Attribute` "/Script/IronEgg.SAttributeSet:MaxStamina" :`AttributeOwner` "/Script/CoreUObject.Class'\"/Script/IronEgg.SAttributeSet\"'")))
  (bind _aswbp_health (cast `/Game/Blueprint/WBP_Health` (`WidgetComponent.GetUserWidgetObject` (`self.Widget`)) :!label _label))
  (`/Engine/EditorBlueprintResources/StandardMacros.IsValid` _returnvalue
    (:`Is Valid`
      (`/Game/Blueprint/WBP_Health.SetHealthProress` _aswbp_health (/ _returnvalue_5 _returnvalue_4) (`KismetTextLibrary.Conv_DoubleToText` _returnvalue_5 "HalfToEven"))
      (`/Game/Blueprint/WBP_Health.SetManaProress` _aswbp_health (/ _returnvalue_6 _returnvalue_3) (`KismetTextLibrary.Conv_DoubleToText` _returnvalue_6 "HalfToEven"))
      (`/Game/Blueprint/WBP_Health.SetStaminaProress` _aswbp_health (/ _returnvalue_2 _returnvalue_7) (`KismetTextLibrary.Conv_DoubleToText` _returnvalue_2 "HalfToEven"))
      (bind (_asynctaskproxy _attribute _newvalue) (`AsyncTaskAttributeChanged.ListenForAttributesChange` _returnvalue (`|MakeArray` (struct :`AttributeName` "Health" :`Attribute` "/Script/IronEgg.SAttributeSet:Health" :`AttributeOwner` "/Script/CoreUObject.Class'\"/Script/IronEgg.SAttributeSet\"'") (struct :`AttributeName` "MaxHealth" :`Attribute` "/Script/IronEgg.SAttributeSet:MaxHealth" :`AttributeOwner` "/Script/CoreUObject.Class'\"/Script/IronEgg.SAttributeSet\"'") (struct :`AttributeName` "Mana" :`Attribute` "/Script/IronEgg.SAttributeSet:Mana" :`AttributeOwner` "/Script/CoreUObject.Class'\"/Script/IronEgg.SAttributeSet\"'") (struct :`AttributeName` "MaxMana" :`Attribute` "/Script/IronEgg.SAttributeSet:MaxMana" :`AttributeOwner` "/Script/CoreUObject.Class'\"/Script/IronEgg.SAttributeSet\"'") (struct :`AttributeName` "Stamina" :`Attribute` "/Script/IronEgg.SAttributeSet:Stamina" :`AttributeOwner` "/Script/CoreUObject.Class'\"/Script/IronEgg.SAttributeSet\"'") (struct :`AttributeName` "MaxStamina" :`Attribute` "/Script/IronEgg.SAttributeSet:MaxStamina" :`AttributeOwner` "/Script/CoreUObject.Class'\"/Script/IronEgg.SAttributeSet\"'") :!type "GameplayAttribute Structure"))
        (:`OnAttributeChanged`
          (`|ExecutionSequence`
            (:`then_0`
              (if (== _attribute (struct :`AttributeName` "Health" :`Attribute` "/Script/IronEgg.SAttributeSet:Health" :`AttributeOwner` "/Script/CoreUObject.Class'\"/Script/IronEgg.SAttributeSet\"'"))
                (`/Game/Blueprint/WBP_Health.SetHealthProress` _aswbp_health (/ _newvalue _returnvalue_4) (`KismetTextLibrary.Conv_DoubleToText` _newvalue "HalfToEven"))))
            (:`then_1`
              (if (== _attribute (struct :`AttributeName` "Mana" :`Attribute` "/Script/IronEgg.SAttributeSet:Mana" :`AttributeOwner` "/Script/CoreUObject.Class'\"/Script/IronEgg.SAttributeSet\"'"))
                (`/Game/Blueprint/WBP_Health.SetManaProress` _aswbp_health (/ _newvalue _returnvalue_3) (`KismetTextLibrary.Conv_DoubleToText` _newvalue "HalfToEven"))))
            (:`then_2`
              (if (== _attribute (struct :`AttributeName` "Stamina" :`Attribute` "/Script/IronEgg.SAttributeSet:Stamina" :`AttributeOwner` "/Script/CoreUObject.Class'\"/Script/IronEgg.SAttributeSet\"'"))
                (`/Game/Blueprint/WBP_Health.SetStaminaProress` _aswbp_health (/ _newvalue _returnvalue_7) (`KismetTextLibrary.Conv_DoubleToText` _newvalue "HalfToEven"))))))))))

(event `初始化血条`
  (goto _label))

(event `self.OnPlayerStateClient_Implementation`
  (`self.初始化血条`))

(event `self.OnPossesseServer_Implementation`
  (`self.初始化技能效果`)
  (`self.初始化血条`))

(fn `UserConstructionScript`)

(fn `获取技能组件`
  (returns (ReturnValue :type "SAbilitySystemComponent Object Reference"))
  (bind _assplayer_state (cast `SPlayerState` (`self.PlayerState`))
    (:`then`
      (return (`SPlayerState.GetSAbilitySystemComponent` _assplayer_state)))
    (:`CastFailed`
      (return null))))